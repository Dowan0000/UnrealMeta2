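; BP_MyPawn is a Pawn that prints elapsed play time on screen as zero-padded minutes and seconds with Korean unit labels (분, 초).
; Tick feeds delta time into DeltaSecToString, which accumulates the total and formats it through FloatToStr00, printing only when the string changes.
; BeginPlay briefly prints the pawn's display name, and disconnected float math and comparison nodes remain unused in the graph.
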(event EventBeginPlay
  (Development|PrintString (Utilities|GetDisplayName self) true true "(R=0.000000,G=0.660000,B=1.000000,A=1.000000)" 0.01))

(event Collision|EventActorBeginOverlap
  (params (OtherActor :type Actor%20Object%20Reference)))

(event EventTick
  (params (DeltaSeconds :type Float%20%28single-precision%29))
  ;[1 1 1] DeltaSeconds = 00 분 00 초
  (bind _returnvalue (CallFunction|DeltaSectoString (* DeltaSeconds 1.0)))
  (if (Utilities|Enum|NotEqual(Enum) _returnvalue (Variables|Default|GetCompareStr))
    (bind _output_get (Variables|Default|SetCompareStr _returnvalue))
    (Development|PrintString _output_get true true "(R=0.000000,G=0.660000,B=1.000000,A=1.000000)" 1.0)))

(fn ConstructionScript)

(fn FloattoStr00
  (params (Number :type Float%20%28single-precision%29))
  (bind _returnvalue (Math|Float|Floor Number))
  (bind _returnvalue_2 (Utilities|String|ToString(Integer) _returnvalue))
  (if (< _returnvalue 10)
    (return (Utilities|String|Append "0" _returnvalue_2))
    (else
      (return _returnvalue_2))))

(fn DeltaSectoString
  (params (DeltaSeconds :type Float%20%28single-precision%29))
  (bind _output_get (Variables|Default|SetTotalDeltaSeconds (+ DeltaSeconds (Variables|Default|GetTotalDeltaSeconds))))
  (return (Utilities|String|Append (CallFunction|FloattoStr00 (/ _output_get 6e+01)) "분" (CallFunction|FloattoStr00 (Math|Float|%(Float) _output_get 6e+01)) "초")))